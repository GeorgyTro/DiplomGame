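; BP_Weapom is a weapon item Blueprint for an FPS inventory, built around an AGR_Item component.
; Its event graph prints a formatted debug message with the item name on pickup, hide/show, drop, equip, use and unequip.
; The construction script is empty, leaving an unwired node that would snap EBBarrel to a barrel socket on the skeletal mesh.
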(event OnPickup(AGR_Item)
  (params (Inventory :type AGR%20Inventory%20Manager%20Object%20Reference))
  (Development|PrintText (Utilities|Text|FormatText "{1} : Pick Up by {2}" (Variables|/Script/AGRPRO.AGR_ItemComponent|GetItemName (Variables|Default|GetAGR_Item)) (Guid|ToString(Guid) (Variables|/Script/AGRPRO.AGR_InventoryManager|GetInventoryId Inventory)))))

(event OnHiddenShown(AGR_Item)
  (params (bHidden :type Boolean))
  (Development|PrintText (Utilities|Text|FormatText "{1} - hidden? {2}" (Variables|/Script/AGRPRO.AGR_ItemComponent|GetItemName (Variables|Default|GetAGR_Item)) bHidden)))

(event OnItemDropped(AGR_Item)
  (Development|PrintText (Utilities|Text|FormatText "{1} Dropped!" (Variables|/Script/AGRPRO.AGR_ItemComponent|GetItemName (Variables|Default|GetAGR_Item)))))

(event OnEquip(AGR_Item)
  (params (User :type Actor%20Object%20Reference))
  (Development|PrintText (Utilities|Text|FormatText "{1} Equiped!" (Variables|/Script/AGRPRO.AGR_ItemComponent|GetItemName (Variables|Default|GetAGR_Item)))))

(event OnItemUsed(AGR_Item)
  (params (User :type Actor%20Object%20Reference))
  (Development|PrintText (Utilities|Text|FormatText "{1} Used" (Variables|/Script/AGRPRO.AGR_ItemComponent|GetItemName (Variables|Default|GetAGR_Item)))))

(event OnUnequip(AGR_Item)
  (params (User :type Actor%20Object%20Reference))
  (Development|PrintText (Utilities|Text|FormatText "{1} Unequiped" (Variables|/Script/AGRPRO.AGR_ItemComponent|GetItemName (Variables|Default|GetAGR_Item)))))

(fn ConstructionScript)