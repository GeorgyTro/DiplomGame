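; Top-down player character with WASD movement relative to camera yaw and aiming at the visible mouse cursor.
; Each tick turns control rotation toward the cursor's trace hit, with clamped pitch.
; Holding right mouse switches the AGR anim component from velocity-facing locomotion to desired rotation with a rifle pose.
; Left click plays a jump-idle-land additive montage in the locomotion pose when no montage is playing; click-to-move logic is unconnected.
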(event EventBeginPlay
  ;[1 1 1] Begin show cursor
  (Variables|/Script/Engine.PlayerController|SetbShowMouseCursor (Game|GetPlayerController 0) true))

(event EventTick
  (params (DeltaSeconds :type Float%20%28single-precision%29))
  (bind _returnvalue (Transformation|GetActorLocation))
  (bind _returnvalue_2 (Game|GetPlayerController 0))
  (bind _hitresult (Game|Player|GetHitResultUnderCursorbyChannel _returnvalue_2 "TraceTypeQuery1" true))
  (bind _impactpoint (Collision|BreakHitResult _hitresult))
  (bind _returnvalue_3 (Math|Rotator|FindLookatRotation _returnvalue _impactpoint))
  ;[1 1 1] Смотреть за мышью
  (if true
    (Pawn|SetControlRotation _returnvalue_2 (Math|Rotator|MakeRotator (.roll _returnvalue_3) (Math|Float|Clamp(Float) (.pitch _returnvalue_3) -3e+01 56.0) (.yaw _returnvalue_3)))))

(event Input|AxisEvents|InputAxisMoveForward
  (params (AxisValue :type Float%20%28single-precision%29))
  (bind _charactermovement (Variables|Character|GetCharacterMovement))
  ;[1 1 1] wasd imput
  (if (>= (Math|Float|Absolute(Float) AxisValue) 0.1)
    (Class|NavMovementComponent|StopActiveMovement _charactermovement)
    (Class|PawnMovementComponent|AddInputVector _charactermovement (* (Math|Vector|GetForwardVector (Math|Rotator|MakeRotator 0.0 0.0 (.yaw (Transformation|GetWorldRotation (Variables|Default|GetCamera))))) AxisValue) false)))

(event Input|AxisEvents|InputAxisMoveRight
  (params (AxisValue :type Float%20%28single-precision%29))
  (bind _charactermovement (Variables|Character|GetCharacterMovement))
  ;[1 1 1] wasd imput
  (if (>= (Math|Float|Absolute(Float) AxisValue) 0.1)
    (Class|NavMovementComponent|StopActiveMovement _charactermovement)
    (Class|PawnMovementComponent|AddInputVector _charactermovement (* (Math|Vector|GetRightVector (Math|Rotator|MakeRotator 0.0 0.0 (.yaw (Transformation|GetWorldRotation (Variables|Default|GetCamera))))) AxisValue) false)))

(event Input|MouseEvents|LeftMouseButton
  (params (Key :type Key%20Structure :default "None"))
  ;[1 1 1] Идти за мышью
)

(event Input|MouseEvents|RightMouseButton
  (params (Key :type Key%20Structure :default "None"))
  (bind _agranimmastercomponent (Variables|Default|GetAGRAnimMasterComponent))
  (:Pressed
    (Class|AGRAnimMasterComponent|SetupRotation _agranimmastercomponent "DesiredRotation" 3.6e+02 9e+01 5.0)
    (Class|AGRAnimMasterComponent|SetupBasePose _agranimmastercomponent "(TagName=\"Animation Base.RiflePro\")"))
  (:Released
    (Class|AGRAnimMasterComponent|SetupRotation _agranimmastercomponent "RotateToVelocity" 3.6e+02 9e+01 5.0)
    (Class|AGRAnimMasterComponent|SetupBasePose _agranimmastercomponent "(TagName=\"Animation Base.locomotionPro\")")))

(event Input|MouseEvents|LeftMouseButton
  (params (Key :type Key%20Structure :default "None"))
  (:Pressed
    (if (and (not (Class|AnimInstance|IsAnyMontagePlaying (Components|SkeletalMesh|GetAnimInstance (Variables|Character|GetMesh)))) (== (Variables|/Script/AGRPRO.AGRAnimMasterComponent|GetOverlayPose (Variables|Default|GetAGRAnimMasterComponent)) "(TagName=\"Animation Base.locomotionPro\")"))
      (Animation|Montage|PlayMontage (Variables|Character|GetMesh) "/Game/MovementAnimsetPro/Animations/InPlace/JumpIdleLand_Additive_Montage.JumpIdleLand_Additive_Montage"))))

(fn ConstructionScript)