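; Top-down player character that moves by input axes or click-to-move and can aim at the mouse cursor.
; Axis input moves it relative to camera yaw, while left click sends it to the cursor hit point via SimpleMoveToLocation.
; Tick points control rotation at the cursor hit.
; Holding right mouse switches AGRAnimMasterComponent to desired rotation, and releasing returns to rotate-to-velocity, resetting the base pose each time.
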(event EventBeginPlay
  (Variables|/Script/Engine.PlayerController|SetbShowMouseCursor (Game|GetPlayerController 0) true))

(event EventTick
  (params (DeltaSeconds :type Float%20%28single-precision%29))
  (bind _returnvalue (Game|GetPlayerController 0))
  (bind (_hitresult _returnvalue_2) (Game|Player|GetHitResultUnderCursorbyChannel _returnvalue "TraceTypeQuery1" true))
  (if _returnvalue_2
    (Pawn|SetControlRotation _returnvalue (Math|Rotator|FindLookatRotation (Transformation|GetActorLocation) (.ImpactPoint (Collision|BreakHitResult _hitresult))))))

(event Input|AxisEvents|InputAxisMoveForward
  (params (AxisValue :type Float%20%28single-precision%29))
  (Class|PawnMovementComponent|AddInputVector (Variables|Character|GetCharacterMovement) (* (Math|Vector|GetForwardVector (Math|Rotator|MakeRotator 0.0 0.0 (.yaw (Transformation|GetWorldRotation (Variables|Default|GetCamera))))) AxisValue) false))

(event Input|AxisEvents|InputAxisMoveRight
  (params (AxisValue :type Float%20%28single-precision%29))
  (Class|PawnMovementComponent|AddInputVector (Variables|Character|GetCharacterMovement) (* (Math|Vector|GetRightVector (Math|Rotator|MakeRotator 0.0 0.0 (.yaw (Transformation|GetWorldRotation (Variables|Default|GetCamera))))) AxisValue) false))

(event Input|MouseEvents|LeftMouseButton
  (params (Key :type Key%20Structure :default "None"))
  (bind _returnvalue (Game|GetPlayerController 0))
  (bind (_hitresult _returnvalue_2) (Game|Player|GetHitResultUnderCursorbyChannel _returnvalue "TraceTypeQuery1" true))
  ;[1 1 1] Смотреть на мышь
  (:Pressed
    (if _returnvalue_2
      (AI|Navigation|SimpleMovetoLocation _returnvalue (.ImpactPoint (Collision|BreakHitResult _hitresult))))))

(event Input|MouseEvents|RightMouseButton
  (params (Key :type Key%20Structure :default "None"))
  (bind _agranimmastercomponent (Variables|Default|GetAGRAnimMasterComponent))
  (:Pressed
    (Class|AGRAnimMasterComponent|SetupRotation _agranimmastercomponent "DesiredRotation" 3.6e+02 9e+01 5.0)
    (Class|AGRAnimMasterComponent|SetupBasePose _agranimmastercomponent))
  (:Released
    (Class|AGRAnimMasterComponent|SetupRotation _agranimmastercomponent "RotateToVelocity" 3.6e+02 9e+01 5.0)
    (Class|AGRAnimMasterComponent|SetupBasePose)))

(fn ConstructionScript)