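; BP_weapon is an automatic weapon that fires BP_Bullet actors while its trigger is toggled on.
; The Firing event sets CanFire and runs a looping fire sequence that calls SpawnProjectile, then waits on a short fixed Delay between shots.
; A FireDelay flag blocks re-entry during that wait, so repeated toggles cannot bypass the fire rate.
; SpawnProjectile spawns each bullet at the skeletal mesh's Fire_FX_Slot socket transform in world space.
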(event Custom|Firing
  (params (Toggle :type Boolean))
  (bind _output_get (Variables|Default|SetCanFire Toggle))
  (if _output_get
    (if (and (Variables|Default|GetCanFire) (not (Variables|Default|GetFireDelay))) :!label _label
      (Variables|Default|SetFireDelay true)
      (CallFunction|SpawnProjectile)
      (Utilities|FlowControl|Delay 0.1)
      (Variables|Default|SetFireDelay false)
      (goto _label))))

(fn ConstructionScript)

(fn SpawnProjectile
  (Game|SpawnActorfromClass "/Game/TDS/BP_Bullet.BP_Bullet_C" (Transformation|GetSocketTransform (Variables|Default|GetSkeletalMesh) "Fire_FX_Slot" "RTS_World") "Undefined" 0 0))