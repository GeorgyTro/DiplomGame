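; Top-down shooter player character that moves with camera-relative WASD, aims at the mouse cursor and carries an AK47 spawned onto a mesh socket.
; Tick turns control rotation toward the cursor trace hit with clamped pitch.
; Right mouse switches AGR animation rotation between desired and velocity-facing.
; Fire calls the weapon, while R runs a DoOnce-gated montage reload; click-to-move is unconnected and SnapWeapon is empty.
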(event EventBeginPlay
  ;[0 0.8594 1] Begin show cursor
  (Variables|/Script/Engine.PlayerController|SetbShowMouseCursor (Game|GetPlayerController 0) true)
  (bind _returnvalue (Game|SpawnActorfromClass "/Game/TDS/Weapon/AK47.AK47_C" (Math|Transform|MakeTransform "0, 0, 0" "0, 0, 0" "1,1,1") "Undefined" 0 0))
  ;[1 0.9844 0] Comment
  (bind _output_get (Variables|Default|SetPrimary%20weapon _returnvalue))
  (Transformation|AttachComponentToComponent _output_get (Variables|Character|GetMesh) "TDS_Socket" "KeepRelative" "KeepRelative" "KeepRelative" true))

(event EventTick
  (params (DeltaSeconds :type Float%20%28single-precision%29))
  (bind _returnvalue (Transformation|GetActorLocation))
  (bind _returnvalue_2 (Game|GetPlayerController 0))
  (bind _hitresult (Game|Player|GetHitResultUnderCursorbyChannel _returnvalue_2 "TraceTypeQuery1" true))
  (bind _impactpoint (Collision|BreakHitResult _hitresult))
  (bind _returnvalue_3 (Math|Rotator|FindLookatRotation _returnvalue _impactpoint))
  ;[0.1016 1 0] Смотреть за мышью
  (if true
    (Pawn|SetControlRotation _returnvalue_2 (Math|Rotator|MakeRotator (.roll _returnvalue_3) (Math|Float|Clamp(Float) (.pitch _returnvalue_3) -3e+01 56.0) (.yaw _returnvalue_3)))))

(event Input|ActionEvents|InputActionFire
  (params (Key :type Key%20Structure :default "None"))
  (bind _primary_weapon (Variables|Default|GetPrimary%20weapon))
  ;[1 0.3516 0] Comment
  (:Pressed
    (Default|Fire _primary_weapon)
    (if (> (Variables|/Game/TDS/Weapon/Weapon_Base.Weapon_Base_C|GetAmmo_Count _primary_weapon) 0)
      _)))

(event Input|AxisEvents|InputAxisMoveForward
  (params (AxisValue :type Float%20%28single-precision%29))
  (bind _charactermovement (Variables|Character|GetCharacterMovement))
  ;[0.2656 1 0] wasd imput
  (if (>= (Math|Float|Absolute(Float) AxisValue) 0.1)
    (Class|NavMovementComponent|StopActiveMovement _charactermovement)
    (Class|PawnMovementComponent|AddInputVector _charactermovement (* (Math|Vector|GetForwardVector (Math|Rotator|MakeRotator 0.0 0.0 (.yaw (Transformation|GetWorldRotation (Variables|Default|GetCamera))))) AxisValue) false)))

(event Input|AxisEvents|InputAxisMoveRight
  (params (AxisValue :type Float%20%28single-precision%29))
  (bind _charactermovement (Variables|Character|GetCharacterMovement))
  ;[0.2656 1 0] wasd imput
  (if (>= (Math|Float|Absolute(Float) AxisValue) 0.1)
    (Class|NavMovementComponent|StopActiveMovement _charactermovement)
    (Class|PawnMovementComponent|AddInputVector _charactermovement (* (Math|Vector|GetRightVector (Math|Rotator|MakeRotator 0.0 0.0 (.yaw (Transformation|GetWorldRotation (Variables|Default|GetCamera))))) AxisValue) false)))

(event Input|MouseEvents|LeftMouseButton
  (params (Key :type Key%20Structure :default "None"))
  ;[0 0.4375 1] Идти за мышью
)

(event Input|MouseEvents|RightMouseButton
  (params (Key :type Key%20Structure :default "None"))
  (bind _agranimmastercomponent (Variables|Default|GetAGRAnimMasterComponent))
  ;[0.875 0 1] Comment
  (:Pressed
    (Class|AGRAnimMasterComponent|SetupRotation _agranimmastercomponent "DesiredRotation" 3.6e+02 9e+01 5.0)
    (Class|AGRAnimMasterComponent|SetupBasePose _agranimmastercomponent "(TagName=\"Animation Base.RiflePro\")"))
  (:Released
    (Class|AGRAnimMasterComponent|SetupRotation _agranimmastercomponent "RotateToVelocity" 3.6e+02 9e+01 5.0)
    (Class|AGRAnimMasterComponent|SetupBasePose _agranimmastercomponent "(TagName=\"Animation Base.RiflePro\")")))

(event Input|KeyboardEvents|R
  (params (Key :type Key%20Structure :default "None"))
  (bind _primary_weapon (Variables|Default|GetPrimary%20weapon))
  (bind _primary_weapon_2 (Variables|Default|GetPrimary%20weapon))
  (:Pressed
    (if (< (Variables|/Game/TDS/Weapon/Weapon_Base.Weapon_Base_C|GetAmmo_Count _primary_weapon_2) (Variables|/Game/TDS/Weapon/Weapon_Base.Weapon_Base_C|GetMax_Ammo _primary_weapon_2))
      (Utilities|FlowControl|DoOnce false :!label _label
        (:Completed
          (Variables|Default|SetIs_Reload true)
          (Animation|Montage|MontagePlay (Components|SkeletalMesh|GetAnimInstance (Variables|Character|GetMesh)) "/Game/IBFPSStarterPack/Animations/Arms/ANIM_ArK-47_Reload_Montage.ANIM_ArK-47_Reload_Montage" 1.0 "MontageLength" 0.0 true)
          (Default|Reload _primary_weapon)
          (Utilities|FlowControl|Delay (Variables|/Game/TDS/Weapon/Weapon_Base.Weapon_Base_C|GetReload_Time _primary_weapon))
          (Variables|Default|SetIs_Reload false)
          (goto _label Reset))))))

(fn ConstructionScript)

(fn SnapWeapon)